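; BP-EffectTrigger is a one-shot trigger actor that sets off a heavy effect when a BPAdam actor overlaps it.
; It spawns BPHeavyEffect at its own transform, destroys itself and gives the effect a short lifespan.
; In the ExperimentLevelUser level it also takes a screenshot through the Shot console command.
; A collapse sound node is present but never runs.
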(event EventBeginPlay)

(event Collision|EventActorBeginOverlap
  (params (OtherActor :type Actor%20Object%20Reference))
  (if (Utilities|ClassIsChildOf (Utilities|GetClass OtherActor) "/Game/Blueprints/BP-Adam.BP-Adam_C")
    (bind _returnvalue (Game|SpawnActorfromClass "/Game/Blueprints/BP-HeavyEffect.BP-HeavyEffect_C" (Transformation|GetActorTransform) "Undefined" 0 0))
    (Actor|DestroyActor)
    (Actor|SetLifeSpan _returnvalue 3.0)
    (bind _returnvalue_2 (Game|GetCurrentLevelName true))
    (if (Utilities|Enum|Equal(Enum) _returnvalue_2 "ExperimentLevelUser")
      (Development|ExecuteConsoleCommand "Shot") ; Take Photo
    )))

(event EventTick
  (params (DeltaSeconds :type Float%20%28single-precision%29)))

(fn ConstructionScript)