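; BP-Adam is a controllable pawn Blueprint that moves and fires projectiles.
; MoveForward and StrafeLeft axis inputs add movement along the control rotation's forward and right vectors.
; Pressing ShootWeaponB spawns a BPProjectile offset ahead of the actor by FrontThrow, oriented to the control rotation.
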(event EventBeginPlay)

(event Collision|EventActorBeginOverlap
  (params (OtherActor :type Actor%20Object%20Reference)))

(event EventTick
  (params (DeltaSeconds :type Float%20%28single-precision%29)))

(event Input|ActionEvents|InputActionShootWeaponB
  (params (Key :type Key%20Structure :default "AnyKey"))
  (bind _returnvalue (Pawn|GetControlRotation :!class /Script/Engine.Pawn))
  ;[1 1 1] Shoot_Input
  (:Pressed
    (Game|SpawnActorfromClass "/Game/Blueprints/BP-Projectile.BP-Projectile_C" (Math|Transform|MakeTransform (+ (Transformation|GetActorLocation) (* (Math|Vector|GetForwardVector _returnvalue) (Variables|Default|GetfrontThrow))) _returnvalue) "Undefined" 0 0)))

(event Input|AxisEvents|InputAxisMoveForward
  (params (AxisValue :type Float%20%28single-precision%29))
  ;[1 1 1] Movement_Input
  (Pawn|Input|AddMovementInput (Math|Vector|GetForwardVector (Pawn|GetControlRotation :!class /Script/Engine.Pawn)) AxisValue false))

(event Input|AxisEvents|InputAxisStrafeLeft
  (params (AxisValue :type Float%20%28single-precision%29))
  ;[1 1 1] Movement_Input
  (Pawn|Input|AddMovementInput (Math|Vector|GetRightVector (Pawn|GetControlRotation :!class /Script/Engine.Pawn)) AxisValue false))

(fn ConstructionScript)