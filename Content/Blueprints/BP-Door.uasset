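; Door actor Blueprint that toggles between its starting rotation and a 90-degree yaw turn.
; BeginPlay stores the initial rotation, and each OpenDoor call checks the Turned flag, either adding the yaw with physics teleport or restoring the stored rotation, then flips the flag.
; The rotation snaps without interpolation, and nothing in this Blueprint calls OpenDoor.
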(event EventBeginPlay
  (Variables|Default|SetinitialRotator (Transformation|GetActorRotation)))

(event Collision|EventActorBeginOverlap
  (params (OtherActor :type Actor%20Object%20Reference)))

(event EventTick
  (params (DeltaSeconds :type Float%20%28single-precision%29)))

(fn ConstructionScript)

(fn OpenDoor
  (bind _returnvalue (Transformation|GetActorRotation))
  (bind (_roll _pitch _yaw) (Math|Rotator|BreakRotator _returnvalue))
  (if (Variables|Default|Getturned)
    (Transformation|SetActorRotation (Math|Rotator|MakeRotator _roll _pitch (+ _yaw 9e+01)) true)
    (Variables|Default|Setturned false)
    (else
      (Transformation|SetActorRotation (Variables|Default|GetinitialRotator))
      (Variables|Default|Setturned true))))